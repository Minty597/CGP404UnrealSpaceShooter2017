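; Asteroid actor that drifts along its negative up vector each tick at a set speed.
; When a projectile overlaps it, it spawns an explosion, adds its point value to the player spaceship's score, and destroys both itself and the projectile.
; When it overlaps the spaceship instead, it hides the ship's craft component, explodes and destroys itself.
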(event `self.ReceiveActorBeginOverlap`
  (params (OtherActor :type "Actor Object Reference"))
  (bind _asbp_projectile (cast `/Game/BP_Projectile` OtherActor)
    (:`then`
      (`self.SpaentNewExplosion`)
      (bind _asbp_space_ship (cast `/Game/BP_SpaceShip` (`GameplayStatics.GetPlayerPawn` 0)))
      (set `/Game/BP_SpaceShip.I_Points` (+ (`/Game/BP_SpaceShip.I_Points` _asbp_space_ship) (`self.I_Points`)) _asbp_space_ship)
      (`self.K2_DestroyActor` _asbp_projectile)
      (`self.K2_DestroyActor`))
    (:`CastFailed`
      (bind _asbp_space_ship_2 (cast `/Game/BP_SpaceShip` OtherActor))
      (`SceneComponent.SetHiddenInGame` (`/Game/BP_SpaceShip.SpaceCraft` _asbp_space_ship_2) true true)
      (`self.SpaentNewExplosion`)
      (`self.K2_DestroyActor`))))

(event `self.ReceiveTick`
  (params (DeltaSeconds :type "Float (single-precision)"))
  (`self.K2_AddActorWorldOffset` (* (`SceneComponent.GetUpVector` (`self.DefaultSceneRoot`)) (* (* (`self.F_Speed`) DeltaSeconds) -1.0))))

(fn `SpaentNewExplosion`
  (`GameplayStatics.SpawnEmitterAtLocation` "/Game/StarterContent/Particles/P_Explosion.P_Explosion" (`SceneComponent.K2_GetComponentLocation` (`self.DefaultSceneRoot`)))
  (return))

(fn `UserConstructionScript`)