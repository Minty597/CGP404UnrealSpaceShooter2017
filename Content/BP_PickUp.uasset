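; BP_PickUp is a drifting weapon pickup that swaps the weapon of a BP_SpaceShip that overlaps it.
; On BeginPlay it picks a random class from AvailableWeapons, and Tick moves it along its negative up vector at FSpeed.
; On overlap it destroys the ship's CurrentWeapon, spawns the picked class at the ship's root transform and stores it as CurrentWeapon.
; The graph neither attaches the new weapon nor destroys the pickup.
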(event `self.ReceiveBeginPlay`
  (bind _availableweapons (`self.AvailableWeapons`))
  (set `self.WeaponPickRef` (`KismetArrayLibrary.Array_Get` _availableweapons (`KismetMathLibrary.RandomIntegerInRange` 0 (- (`KismetArrayLibrary.Array_Length` _availableweapons) 1)))))

(event `self.ReceiveActorBeginOverlap`
  (params (OtherActor :type "Actor Object Reference"))
  (bind _asbp_space_ship (cast `/Game/BP_SpaceShip` OtherActor))
  (`self.K2_DestroyActor` (`/Game/BP_SpaceShip.CurrentWeapon` _asbp_space_ship))
  (bind _returnvalue (`|SpawnActorFromClass` (`self.WeaponPickRef`) (`SceneComponent.K2_GetComponentToWorld` (`/Game/BP_SpaceShip.DefaultSceneRoot` _asbp_space_ship)) "Undefined" "OverrideRootScale"))
  (set `/Game/BP_SpaceShip.CurrentWeapon` _returnvalue _asbp_space_ship))

(event `self.ReceiveTick`
  (params (DeltaSeconds :type "Float (single-precision)"))
  (`self.K2_AddActorWorldOffset` (* (`SceneComponent.GetUpVector` (`self.DefaultSceneRoot`)) (* (* (`self.F_Speed`) DeltaSeconds) -1.0))))

(fn `UserConstructionScript`)