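; BP_MiniGun is an automatic weapon that fires projectiles continuously between Shoot and StopShoot calls.
; Shoot calls the parent implementation, stores the passed PlayRef and sets a shooting flag, which StopShoot clears.
; While the flag is set, Tick runs a Delay that throttles the fire rate, then spawns a Projectile at the stored reference's world transform.
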(event `self.ReceiveTick`
  (params (DeltaSeconds :type "Float (single-precision)"))
  (if (`self.B_IsShooting`)
    (`KismetSystemLibrary.Delay` (`self.F_DelayTime`))
    (`|SpawnActorFromClass` (`self.Projectile`) (`SceneComponent.K2_GetComponentToWorld` (`self.Playref`)) "Undefined" "OverrideRootScale")))

(event `self.Shoot`
  (params (PlayRef :type "StaticMeshComponent Object Reference"))
  (`parent.Shoot` PlayRef)
  (set `self.B_IsShooting` true)
  (set `self.Playref` PlayRef))

(event `self.StopShoot`
  (set `self.B_IsShooting` false))

(fn `UserConstructionScript`)