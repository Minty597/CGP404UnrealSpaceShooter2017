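; BP_ObjectSpawner is an actor that repeatedly spawns ObjectToSpawn at random points inside a box volume.
; Tick feeds a Delay of FWaitTime, which ignores calls while counting down and so acts as a repeating spawn timer.
; Each spawn adds a random offset within the Box component's scaled extents to its world location, without applying the box's rotation.
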(event `self.ReceiveTick`
  (params (DeltaSeconds :type "Float (single-precision)"))
  (bind _x (.x (`BoxComponent.GetScaledBoxExtent` (`self.Box`))))
  (bind _y (.y (`BoxComponent.GetScaledBoxExtent` (`self.Box`))))
  (bind _z (.z (`BoxComponent.GetScaledBoxExtent` (`self.Box`))))
  (`KismetSystemLibrary.Delay` (`self.F_waitTime`))
  (`|SpawnActorFromClass` (`self.ObjectToSpawn`) (`KismetMathLibrary.Conv_VectorToTransform` (+ (`SceneComponent.K2_GetComponentLocation` (`self.Box`)) (`KismetMathLibrary.MakeVector` (`KismetMathLibrary.RandomFloatInRange` (* -1 _x) _x) (`KismetMathLibrary.RandomFloatInRange` (* -1 _y) _y) (`KismetMathLibrary.RandomFloatInRange` (* -1 _z) _z)))) "Undefined" "OverrideRootScale"))

(fn `UserConstructionScript`)